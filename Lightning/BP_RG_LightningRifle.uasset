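; Lightning rifle weapon for RocketGib characters in Unreal Tournament, with a refire cooldown based on when it last started firing.
; Firing records the time and shows a cooldown alert on the player's HUD.
; On bring-up, if the character's CanFireLightning flag is off, it disables weapon firing, then re-enables it immediately or by timer once the remaining refire time runs out, refreshing the alert while waiting.
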(event `self.OnStartedFiring`
  (set `self.LastFiredTime` (`GameplayStatics.GetTimeSeconds`))
  (`self.UpdateHUD` 0.75))

(event `self.OnBringUp`
  (bind _rgcharacter (`self.GetCharacter`))
  (if (not (`/Game/dc/RocketGib/RocketGibCharacter.CanFireLightning` _rgcharacter))
    (`/Game/dc/RocketGib/Lib/LibWeaponDisabler.DisableWeaponFiring` _rgcharacter)
    (`self.StartRefireTimer`)))

(event `StartRefireTimer`
  (bind _timeleft (`self.TimeUntilRefire`))
  (if (> _timeleft 0.0)
    (`KismetSystemLibrary.K2_SetTimerDelegate` (delegate `ReAllowFiring`) _timeleft)
    (`self.UpdateHUD` 0.0)
    (else
      (`self.ReAllowFiring`))))

(event `ReAllowFiring`
  (`/Game/dc/RocketGib/Lib/LibWeaponDisabler.EnableWeaponFiring` (`self.GetCharacter`)))

(fn `GetCharacter`
  (returns (RGCharacter :type "/Game/dc/RocketGib/RocketGibCharacter Object Reference"))
  (bind _asrocket_gib_character (cast `/Game/dc/RocketGib/RocketGibCharacter` (`self.GetOwner`))
    (:`then`
      _)
    (:`CastFailed`
      _))
  (return _asrocket_gib_character))

(fn `TimeUntilRefire`
  (returns (TimeLeft :type "Float (double-precision)"))
  (bind _returnvalue (`self.GetRefireTime` 0))
  (return (- (+ (`self.LastFiredTime`) _returnvalue) (`GameplayStatics.GetTimeSeconds`))))

(fn `UpdateHUD`
  (params (TimeToNotify :type "Float (double-precision)"))
  (bind _asutplayer_controller (cast `UTPlayerController` (`self.GetOwner` (`self.GetOwner`))))
  (`/Engine/EditorBlueprintResources/StandardMacros.IsValid` _asutplayer_controller
    (:`Is Valid`
      (bind (_hud _valid) (`/Game/dc/RocketGib/Lib/LibRocketGibHUD.GetHUDRef` _asutplayer_controller))
      (if _valid
        (`/Game/dc/RocketGib/Lib/RGHudInterface.ShowCooldownAlert` _hud (`self.TimeUntilRefire`) TimeToNotify)))))

(fn `UserConstructionScript`)
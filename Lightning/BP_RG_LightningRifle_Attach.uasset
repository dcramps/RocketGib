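; Lightning rifle attachment Blueprint that manages the visuals for its powered glow and flare.
; The construction script creates a dynamic soft glow dot material, which BeginPlay applies to several PoweredGlow material slots and brightens.
; A fast looping timer polls whether PoweredGlow is active, switching the flare particle effect on or off to match and zeroing its relative roll and yaw while active.
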(event `self.ReceiveBeginPlay`
  (bind _poweredglow (`self.PoweredGlow`))
  (bind _chargedglow (`self.ChargedGlow`))
  (`KismetSystemLibrary.K2_SetTimerDelegate` (delegate `CheckGlow`) 0.05 true)
  (`PrimitiveComponent.SetMaterial` _poweredglow 2 _chargedglow)
  (`PrimitiveComponent.SetMaterial` _poweredglow 3 _chargedglow)
  (`PrimitiveComponent.SetMaterial` _poweredglow 4 _chargedglow)
  (`MaterialInstanceDynamic.SetScalarParameterValue` (`self.ChargedGlow`) "DistantBrightness" 5.0))

(event `CheckGlow`
  (bind _pfx_powered_flare (`self.PFX_Powered_Flare`))
  (bind _pfx_powered_flare_2 (`self.PFX_Powered_Flare`))
  (if (`ActorComponent.IsActive` (`self.PoweredGlow`))
    (`ActorComponent.Activate` _pfx_powered_flare false)
    (`SceneComponent.K2_SetRelativeRotation` _pfx_powered_flare_2 (`KismetMathLibrary.MakeRotator` 0.0 (.pitch (`SceneComponent.RelativeRotation` _pfx_powered_flare_2))) false false)
    (else
      (`ActorComponent.Deactivate` _pfx_powered_flare))))

(fn `UserConstructionScript`
  (bind _returnvalue (`KismetMaterialLibrary.CreateDynamicMaterialInstance` "/Game/RestrictedAssets/Weapons/LightningRifle/Assets/Materials/M_SoftGlowDot_01_Inst.M_SoftGlowDot_01_Inst"))
  (set `self.ChargedGlow` _returnvalue))
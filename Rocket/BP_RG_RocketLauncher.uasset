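; BP_RG_RocketLauncher is the rocket launcher weapon for RocketGib characters, built on Unreal Tournament classes.
; Starting to fire notifies the owning RocketGibCharacter through RocketFired.
; Bringing the weapon up enables weapon firing, clears the character's CanFireLightning flag and calls ShowCooldownAlert on the player's HUD with negative times.
; A GetCharacter helper casts the weapon's owner to RocketGibCharacter for both events.
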(event `self.OnStartedFiring`
  (`/Game/dc/RocketGib/RocketGibCharacter.RocketFired` (`self.GetCharacter`)))

(event `self.OnBringUp`
  (bind _rgcharacter (`self.GetCharacter`))
  (`/Game/dc/RocketGib/Lib/LibWeaponDisabler.EnableWeaponFiring` _rgcharacter)
  (set `/Game/dc/RocketGib/RocketGibCharacter.CanFireLightning` false _rgcharacter)
  (bind _asutplayer_controller (cast `UTPlayerController` (`self.GetOwner` _rgcharacter)))
  (bind _hud (`/Game/dc/RocketGib/Lib/LibRocketGibHUD.GetHUDRef` _asutplayer_controller))
  (`/Game/dc/RocketGib/Lib/RGHudInterface.ShowCooldownAlert` _hud -1.0 -1.0))

(fn `GetCharacter`
  (returns (RGCharacter :type "/Game/dc/RocketGib/RocketGibCharacter Object Reference"))
  (bind _asrocket_gib_character (cast `/Game/dc/RocketGib/RocketGibCharacter` (`self.GetOwner`))
    (:`then`
      _)
    (:`CastFailed`
      _))
  (return _asrocket_gib_character))

(fn `UserConstructionScript`)